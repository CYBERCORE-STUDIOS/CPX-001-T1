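; PlayerAlpha is a player pawn Blueprint that provides basic look and movement controls.
; Look axis inputs feed controller yaw and pitch directly.
; Movement axis inputs feed AddMovementInput along the Camera component's forward and right vectors, so travel follows the camera's orientation, with forward not flattened to the ground plane.
; BeginPlay, overlap and the construction script are empty.
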(event `InputAxis|Look Side`
  (params (AxisValue :type "Float (single-precision)"))
  ;[1 1 1] CAM Movement
  ;;[1 1 1] Look Side
  (`self.AddControllerYawInput` AxisValue))

(event `InputAxis|Look Up`
  (params (AxisValue :type "Float (single-precision)"))
  ;[1 1 1] CAM Movement
  ;;[1 1 1] Look Up / Down
  (`self.AddControllerPitchInput` AxisValue))

(event `InputAxis|Forward / Backward Movement`
  (params (AxisValue :type "Float (single-precision)"))
  ;[1 1 1] Player Movement
  ;;[1 1 1] Forward / Backward Movement
  (`self.AddMovementInput` (`SceneComponent.GetForwardVector` (`self.Camera`)) AxisValue))

(event `InputAxis|Side Movement`
  (params (AxisValue :type "Float (single-precision)"))
  ;[1 1 1] Player Movement
  ;;[1 1 1] Side Movement
  (`self.AddMovementInput` (`SceneComponent.GetRightVector` (`self.Camera`)) AxisValue))

(fn `UserConstructionScript`)